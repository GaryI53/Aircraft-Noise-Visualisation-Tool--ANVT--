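; Player-flown aircraft Blueprint with simple physics-based flight, driven by torques and velocity on its Collision component.
; Mouse axes apply pitch and roll torque, weaker at zero throttle, while Move Right applies throttle-scaled yaw.
; A looping timer ramps throttle from held W/S keys.
; Tick applies counter-rotation torque and downward force, blends velocity toward forward vector times throttle, and interpolates throttle down when ZeroThrottle is set.
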(event `InputAxisKey|MouseY`
  (params (AxisValue :type "Float (single-precision)"))
  (bind _returnvalue (* AxisValue 120.0))
  (set `self.MouseY` AxisValue)
  (`PrimitiveComponent.AddTorqueInDegrees` (`self.Collision`) (`KismetMathLibrary.VLerp` (0.0 0.0 0.0) (* (`SceneComponent.GetRightVector` (`self.Collision`)) (`KismetMathLibrary.SelectFloat` _returnvalue (/ _returnvalue 3.0) (> (`self.CurrentThrottle`) 0.0))) 0.1) "None" true))

(event `InputAxisKey|MouseX`
  (params (AxisValue :type "Float (single-precision)"))
  (bind _returnvalue (* AxisValue -120.0))
  (set `self.MouseX` AxisValue)
  (`PrimitiveComponent.AddTorqueInDegrees` (`self.Collision`) (`KismetMathLibrary.VLerp` (0.0 0.0 0.0) (* (`SceneComponent.GetForwardVector` (`self.Collision`)) (`KismetMathLibrary.SelectFloat` _returnvalue (/ _returnvalue 3.0) (> (`self.CurrentThrottle`) 0.0))) 0.1) "None" true))

(event `InputAxis|Move Right`
  (params (AxisValue :type "Float (single-precision)"))
  (bind _returnvalue (/ (`self.CurrentThrottle`) 2500.0))
  (set `self.Rudder` (* AxisValue _returnvalue))
  (`PrimitiveComponent.AddTorqueInDegrees` (`self.Collision`) (`KismetMathLibrary.VLerp` (0.0 0.0 0.0) (* (`SceneComponent.GetUpVector` (`self.Collision`)) (* (* AxisValue 250.0) _returnvalue)) 0.1) "None" true))

(event `self.ReceiveBeginPlay`
  (`KismetSystemLibrary.K2_SetTimer` null "Throttle" 0.025 true))

(event `self.ReceiveTick`
  (params (DeltaSeconds :type "Float (single-precision)"))
  (bind _collision (`self.Collision`))
  (`|ExecutionSequence`
    (:`then_0`
      (`PrimitiveComponent.AddTorqueInDegrees` _collision (/ (`KismetMathLibrary.NegateVector` (`PrimitiveComponent.GetPhysicsAngularVelocityInDegrees` (`self.Collision`) "None")) (0.75 0.0 0.0)) "None" false)
      (`PrimitiveComponent.AddForce` _collision (0.0 0.0 -1500.0) "None" false)
      (`self.speed`))
    (:`then_1`
      (if (`self.ZeroThrottle`)
        (set `self.CurrentThrottle` (`KismetMathLibrary.FInterpTo_Constant` (`self.CurrentThrottle`) 0.0 (`GameplayStatics.GetWorldDeltaSeconds`) 800.0))))))

(event `Key|W`
  (params (Key :type "Key Structure"))
  (:`Pressed`
    (set `self.MoveThrottleUp` true))
  (:`Released`
    (set `self.MoveThrottleUp` false)))

(event `Key|S`
  (params (Key :type "Key Structure"))
  (:`Pressed`
    (set `self.MoveThrottleDown` true))
  (:`Released`
    (set `self.MoveThrottleDown` false)))

(fn `speed`
  (bind _returnvalue (`PrimitiveComponent.GetPhysicsLinearVelocity` (`self.Collision`) "None"))
  (`PrimitiveComponent.SetPhysicsLinearVelocity` (`self.Collision`) (`KismetMathLibrary.VLerp` _returnvalue (* (`SceneComponent.GetForwardVector` (`self.Collision`)) (* (`self.CurrentThrottle`) 200.0)) 0.1) false "None"))

(fn `Throttle`
  (`|ExecutionSequence`
    (:`then_0`
      (if (`self.MoveThrottleUp`)
        (set `self.CurrentThrottle` (`KismetMathLibrary.FClamp` (+ (`self.CurrentThrottle`) 1.5) 0.0 125.0))
        (elif (`self.MoveThrottleDown`)
          (if (> (`self.CurrentThrottle`) 50.0)
            (set `self.CurrentThrottle` (`KismetMathLibrary.FClamp` (+ (`self.CurrentThrottle`) -0.5) 0.0 125.0))))))))

(fn `UserConstructionScript`)